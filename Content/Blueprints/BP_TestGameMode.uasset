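; Test game mode that spawns dungeon enemies and the boss.
; SpawnNewEnemy runs an EQS query for spawn locations, picked from the best 25%, then spawns a randomly chosen bear or spider at each returned location.
; SpawnBoss checks the dungeon GameState for the boss wave, then after a short delay spawns the boss with an advanced AI behavior tree at a preset location.
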(event Custom|OnQueryFinishedEvent_Event_0
  (params (QueryInstance :type Env%20Query%20Instance%20Blueprint%20Wrapper%20Object%20Reference) (QueryStatus :type EEnvQueryStatus%20Enum :default "Processing"))
  (switch Utilities|FlowControl|Switch|SwitchonEEnvQueryStatus QueryStatus
    (:Success
      (bind _resultlocations (AI|EQS|GetQueryResultsasLocations QueryInstance))
      ;[1 1 1] Basic Enemy 랜덤 스폰
      (bind _output_get (Variables|Default|SetSpawnEnemyNumber (Math|Random|RandomInteger 2)))
      (switch int _output_get
        (:Default
          (Variables|Default|SetSpawnEnemy "/Game/BasicEnemies/Enemy_Spider/BP_EnemySpider.BP_EnemySpider_C" :!label _label))
        (:0
          (Variables|Default|SetSpawnEnemy "/Game/BasicEnemies/Enemy_Bear/BP_EnemyBear.BP_EnemyBear_C"))
        (:1
          (goto _label)))
      (for _array_element _resultlocations
        (AI|SpawnAIFromClass (Variables|Default|GetSpawnEnemy) 0 _array_element "0, 0, 0" false 0)))))

(event EventSpawnNewEnemy
  (bind _returnvalue (AI|EQS|RunEQSQuery "/Game/EnemiesSpawn/EQS_FindSpawnLocation.EQS_FindSpawnLocation" self "RandomBest25Pct"))
  (EventDispatchers|AssignOnQueryFinishedEvent _returnvalue (delegate Custom|OnQueryFinishedEvent_Event_0)))

(event EventSpawnBoss
  (bind _asbp_dungeon_state (Utilities|Casting|CastToBP_DungeonState (Game|GetGameState)))
  (if (Utilities|Enum|Equal(Enum) (Variables|/Script/DungeonTest.DungeonState|GetWaveState _asbp_dungeon_state) "BossWave")
    (Utilities|FlowControl|Delay 3.0)
    (AI|SpawnAIFromClass "/Game/Boss/BP_Boss.BP_Boss_C" "/Game/Boss/AdvancedAI/BT_AdvancedAI.BT_AdvancedAI" (Variables|Default|GetBossSpawnLocation) "0, 0, 0" false 0)
    (Variables|Default|SetbSpawnBoss false)))

(fn ConstructionScript)